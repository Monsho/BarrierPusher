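; Player pawn that hosts the BarrierPusher game, driving its init, per-frame tick and end.
; A/D set horizontal movement, while Space or left click latches an attack flag that clears each frame.
; Each Tick feeds input and mouse position into TickGame, plays sounds from GameInst cue flags, then draws via RenderGame to a render target.
; Title music stops on the select cue; the push cue has no sound.
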(event `self.ReceiveBeginPlay`
  (`BsGameFunctionLibrary.InitGame` (`self.GameInst`)))

(event `self.ReceiveTick`
  (params (DeltaSeconds :type "Float (single-precision)"))
  (bind _gameinst (`self.GameInst`))
  (bind _returnvalue (`WidgetLayoutLibrary.GetMousePositionOnViewport`))
  (`BsGameFunctionLibrary.TickGame` _gameinst (`self.LeftRightMove`) _returnvalue (`self.PressAttack`))
  (`self.PlaySound`)
  (`BsGameFunctionLibrary.RenderGame` _gameinst (`self.GameAssets`) _returnvalue "/Game/BarrierPusher/RT_Game.RT_Game")
  (set `self.PressAttack` false))

(event `self.ReceiveEndPlay`
  (params (EndPlayReason :type "EEndPlayReason Enum" :default "Destroyed"))
  (`BsGameFunctionLibrary.EndGame` (`self.GameInst`)))

(event `Key|A`
  (params (Key :type "Key Structure"))
  (:`Pressed`
    (set `self.LeftRightMove` -1))
  (:`Released`
    (set `self.LeftRightMove` 0 :!label _label)))

(event `Key|D`
  (params (Key :type "Key Structure"))
  (:`Pressed`
    (set `self.LeftRightMove` 1))
  (:`Released`
    (goto _label)))

(event `Key|SpaceBar`
  (params (Key :type "Key Structure"))
  (:`Pressed`
    (set `self.PressAttack` true :!label _label_2)))

(event `Key|LeftMouseButton`
  (params (Key :type "Key Structure"))
  (:`Pressed`
    (goto _label_2)))

(fn `PlaySound`
  (bind _titlebgm (`self.TitleBGM`))
  (bind (_titlebgm_2 _gameoverbgm _selectse _shotse _bombse _reflectse _pushse) (break `BsGameInstance` (`self.GameInst`)))
  (`|ExecutionSequence`
    (:`then_0`
      (if (> _titlebgm_2 0)
        (bind _returnvalue (`GameplayStatics.CreateSound2D` "/Game/BarrierPusher/Sound/title_Cue.title_Cue" 1.0 1.0 0.0 null))
        (bind _output_get (set `self.TitleBGM` _returnvalue))
        (`AudioComponent.Play` _output_get 0.0)))
    (:`then_1`
      (if (> _gameoverbgm 0)
        (`GameplayStatics.PlaySound2D` "/Game/BarrierPusher/Sound/gameover.gameover" 1.0 1.0 0.0 null null)))
    (:`then_2`
      (if (> _selectse 0)
        (`GameplayStatics.PlaySound2D` "/Game/BarrierPusher/Sound/select.select" 1.0 1.0 0.0 null null)
        (`/Engine/EditorBlueprintResources/StandardMacros.IsValid` _titlebgm
          (:`Is Valid`
            (`AudioComponent.Stop` _titlebgm)))))
    (:`then_3`
      (if (> _shotse 0)
        (`GameplayStatics.PlaySound2D` "/Game/BarrierPusher/Sound/shot.shot" 1.0 1.0 0.0 null null)))
    (:`then_4`
      (if (> _bombse 0)
        (`GameplayStatics.PlaySound2D` "/Game/BarrierPusher/Sound/bomb.bomb" 1.0 1.0 0.0 null null)))
    (:`then_5`
      (if (> _reflectse 0)
        (`GameplayStatics.PlaySound2D` "/Game/BarrierPusher/Sound/reflect.reflect" 1.0 1.0 0.0 null null)))
    (:`then_6`
      (if (> _pushse 0)
        _))))

(fn `UserConstructionScript`)